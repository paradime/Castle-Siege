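; Dawn boss enemy Blueprint that handles the boss's bomb-throw attack and its return to the home position.
; BombThrow moves the boss to Home, then, even if the move fails, turns it toward CombatTarget and plays the BombThrow section of the boss montage.
; ResetCharacter sets MoveToTarget status and moves Home, restoring HomeRotation and Idle status only when the move succeeds.
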(event EventBeginPlay)

(event Collision|EventActorBeginOverlap
  (params (OtherActor :type Actor%20Object%20Reference)))

(event EventTick
  (params (DeltaSeconds :type Float%20%28single-precision%29)))

(event EventResetCharacter
  (bind _self self)
  (bind _self_2 self)
  (Class|Enemy|SetEnemyMovementStatus _self "EMS_MoveToTarget")
  (AI|AIMoveTo _self (Variables|Default|GetHome _self) 0 1.0 false
    (:OnSuccess
      (Transformation|SetActorRotation _self_2 (Variables|Default|GetHomeRotation _self_2))
      (Class|Enemy|SetEnemyMovementStatus _self_2 "EMS_Idle"))))

(event EventBombThrow
  (bind _self self)
  (bind _self_2 self)
  (bind _mesh (Variables|Character|GetMesh _self))
  (bind _returnvalue (Components|SkeletalMesh|GetAnimInstance _mesh))
  (AI|AIMoveTo self (Variables|Default|GetHome) 0 1.0 false
    (:OnSuccess
      _)
    (:OnFail
      _))
  (Transformation|SetActorRotation _self_2 (Math|Rotator|FindLookatRotation (Transformation|GetActorLocation _self_2) (Transformation|GetActorLocation (Variables|Default|GetCombatTarget _self_2))))
  (Animation|Montage|MontagePlay _returnvalue "/Game/Enemies/Boss/Animations/BossAnimMontage.BossAnimMontage" 1.0 "MontageLength" 0.0 true)
  (Ability|Animation|MontageJumptoSection _returnvalue "BombThrow" "/Game/Enemies/Boss/Animations/BossAnimMontage.BossAnimMontage"))

(fn ConstructionScript)